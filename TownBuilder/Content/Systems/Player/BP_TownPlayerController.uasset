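; Player controller for a town-building game that switches between build, move and demolish tools.
; BeginPlay sets game-and-UI input, adds the camera mapping context and activates the start tool.
; SetActiveTool exits the old tool component, swaps its input mapping context for the new tool's, looked up in a per-tool map, then enters the new component and broadcasts the change.
; Input events forward actions to the build and demolish components.
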(event Input|EnhancedActionEvents|EnhancedInputActionIA_CancelHeld
  (params (ActionValue :type Boolean) (ElapsedSeconds :type Float%20%28double-precision%29) (TriggeredSeconds :type Float%20%28double-precision%29) (InputAction :type Input%20Action%20Object%20Reference :default "/Game/Input/IA_CancelHeld.IA_CancelHeld"))
  ;[0 0 0 0.5] Inputs
  ;;[1 1 1 0.5] Move
  (:Started
    (Class|BuildComponent|CancelHeld (Variables|Default|GetBuildComponent))))

(event Input|EnhancedActionEvents|EnhancedInputActionIA_CancelHeld
  (params (ActionValue :type Boolean) (ElapsedSeconds :type Float%20%28double-precision%29) (TriggeredSeconds :type Float%20%28double-precision%29) (InputAction :type Input%20Action%20Object%20Reference :default "/Game/Input/IA_CancelHeld.IA_CancelHeld"))
  ;[0 0 0 0.5] Inputs
  ;;[1 1 1 0.5] Build
  (:Started
    (Class|BuildComponent|CancelHeld (Variables|Default|GetBuildComponent))))

(event Input|EnhancedActionEvents|EnhancedInputActionIA_Demolish
  (params (ActionValue :type Boolean) (ElapsedSeconds :type Float%20%28double-precision%29) (TriggeredSeconds :type Float%20%28double-precision%29) (InputAction :type Input%20Action%20Object%20Reference :default "/Game/Input/IA_Demolish.IA_Demolish"))
  ;[0 0 0 0.5] Inputs
  ;;[1 1 1 0.5] Demolish
  (:Started
    (Class|DemolishComponent|DemolishBuildingUnderCursor (Variables|Default|GetDemolishComponent))))

(event Input|EnhancedActionEvents|EnhancedInputActionIA_PlaceHeld
  (params (ActionValue :type Boolean) (ElapsedSeconds :type Float%20%28double-precision%29) (TriggeredSeconds :type Float%20%28double-precision%29) (InputAction :type Input%20Action%20Object%20Reference :default "/Game/Input/IA_PlaceHeld.IA_PlaceHeld"))
  ;[0 0 0 0.5] Inputs
  ;;[1 1 1 0.5] Build
  (:Started
    (Class|BuildComponent|PlaceHeld (Variables|Default|GetBuildComponent))))

(event Input|EnhancedActionEvents|EnhancedInputActionIA_RotateHeld
  (params (ActionValue :type Float%20%28double-precision%29) (ElapsedSeconds :type Float%20%28double-precision%29) (TriggeredSeconds :type Float%20%28double-precision%29) (InputAction :type Input%20Action%20Object%20Reference :default "/Game/Input/IA_RotateHeld.IA_RotateHeld"))
  ;[0 0 0 0.5] Inputs
  ;;[1 1 1 0.5] Build
  (Class|BuildComponent|RotateHeld (Variables|Default|GetBuildComponent) ActionValue))

(event Input|EnhancedActionEvents|EnhancedInputActionIA_RotateHeld
  (params (ActionValue :type Float%20%28double-precision%29) (ElapsedSeconds :type Float%20%28double-precision%29) (TriggeredSeconds :type Float%20%28double-precision%29) (InputAction :type Input%20Action%20Object%20Reference :default "/Game/Input/IA_RotateHeld.IA_RotateHeld"))
  ;[0 0 0 0.5] Inputs
  ;;[1 1 1 0.5] Move
  (Class|BuildComponent|RotateHeld (Variables|Default|GetBuildComponent) ActionValue))

(event Input|EnhancedActionEvents|EnhancedInputActionIA_PickOrPlaceHeld
  (params (ActionValue :type Boolean) (ElapsedSeconds :type Float%20%28double-precision%29) (TriggeredSeconds :type Float%20%28double-precision%29) (InputAction :type Input%20Action%20Object%20Reference :default "/Game/Input/IA_PickOrPlaceHeld.IA_PickOrPlaceHeld"))
  ;[0 0 0 0.5] Inputs
  ;;[1 1 1 0.5] Move
  (:Started
    (if (Class|BuildComponent|IsHolding (Variables|Default|GetBuildComponent))
      (Class|BuildComponent|PlaceHeld (Variables|Default|GetBuildComponent))
      (else
        (Class|BuildComponent|StartMovingBuildingUnderCursor (Variables|Default|GetBuildComponent))))))

(event EventBeginPlay
  (Utilities|FlowControl|Sequence
    (:then_0
      (Input|SetInputModeGameandUI self 0 "DoNotLock" false false)
      (Input|AddMappingContext (PlayerController|LocalPlayerSubsystems|GetEnhancedInputLocalPlayerSubsystem) "/Game/Input/IMC_CameraMovement.IMC_CameraMovement" 0 "(bIgnoreAllPressedKeysUntilRelease=True,bForceImmediately=False,bNotifyUserSettings=False)"))
    (:then_1
      (CallFunction|SetActiveTool (Variables|Default|GetStartTool)))))

(fn ConstructionScript)

(fn SetActiveTool
  (params (Tool :type ETool%20Enum :default "Manage"))
  (Utilities|FlowControl|Sequence
    (:then_0
      (LocalVariables|SetOldTool (Variables|Default|GetActiveTool))
      (Utilities|IsValid (Variables|Default|GetActiveToolComponent)
        (:Is%20Valid
          (Class|ToolComponent|ExitTool (Variables|Default|GetActiveToolComponent))
          (if (.ReturnValue (Utilities|Map|Find (Variables|Default|GetMappingContextByTool) (LocalVariables|GetOldTool)))
            (Input|RemoveMappingContext (PlayerController|LocalPlayerSubsystems|GetEnhancedInputLocalPlayerSubsystem) (.inputmappingcontext (.Value (Utilities|Map|Find (Variables|Default|GetMappingContextByTool) (LocalVariables|GetOldTool)))) "(bIgnoreAllPressedKeysUntilRelease=True,bForceImmediately=False,bNotifyUserSettings=False)")))))
    (:then_1
      (Variables|Default|SetActiveTool Tool)
      (Input|AddMappingContext (PlayerController|LocalPlayerSubsystems|GetEnhancedInputLocalPlayerSubsystem) (.inputmappingcontext (.Value (Utilities|Map|Find (Variables|Default|GetMappingContextByTool) (Variables|Default|GetActiveTool)))) 1 "(bIgnoreAllPressedKeysUntilRelease=True,bForceImmediately=False,bNotifyUserSettings=False)")
      (bind _output_get (Variables|Default|SetActiveToolComponent (Actor|GetComponentbyClass (.toolcomponent (.Value (Utilities|Map|Find (Variables|Default|GetMappingContextByTool) (Variables|Default|GetActiveTool)))))))
      (Class|ToolComponent|EnterTool _output_get (Variables|Default|GetActiveTool))
      (Default|CallOnActiveToolChanged (Variables|Default|GetActiveTool)))))